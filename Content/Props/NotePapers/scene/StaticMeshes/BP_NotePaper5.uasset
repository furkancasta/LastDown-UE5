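; BP_NotePaper5 is an interactable note paper prop that toggles an on-screen view of note 5.
; Its Interact event alternates through a FlipFlop between opening and closing the WB_Note5 widget, playing a paper sound at the Cube's location each time.
; Opening creates a new widget and ignores player look and move input; closing removes the widget and turns both ignores off.
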(event EventInteract
  (params (PlayerRef :type BP%20First%20Person%20Character%20Object%20Reference))
  (bind _returnvalue (Game|GetPlayerController 0))
  (bind _cube (Variables|Default|GetCube))
  (bind _returnvalue_2 (Transformation|GetWorldLocation _cube))
  (Utilities|FlowControl|FlipFlop
    (:A
      (Audio|PlaySoundatLocation "/Game/Props/NotePapers/scene/StaticMeshes/PaperSound/PaperSound_Cue.PaperSound_Cue" _returnvalue_2 "0, 0, 0" 1.0 1.0 0.0 0 0 0 0)
      (bind _returnvalue_3 (UserInterface|CreateWidget "/Game/Props/NotePapers/scene/StaticMeshes/WB_Note/WB_Note5.WB_Note5_C"))
      (UserInterface|Viewport|AddtoViewport _returnvalue_3 0)
      (Input|SetIgnoreLookInput _returnvalue true)
      (Input|SetIgnoreMoveInput _returnvalue true))
    (:B
      (Audio|PlaySoundatLocation "/Game/Props/NotePapers/scene/StaticMeshes/PaperSound/PaperSound_Cue.PaperSound_Cue" _returnvalue_2 "0, 0, 0" 1.0 1.0 0.0 0 0 0 0)
      (Widget|RemovefromParent _returnvalue_3)
      (Input|SetIgnoreLookInput _returnvalue false)
      (Input|SetIgnoreMoveInput _returnvalue false))))

(fn ConstructionScript)